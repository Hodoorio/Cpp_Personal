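; BP_TableActor is a blackjack table actor that turns keyboard input into game actions.
; Pressing 1, 2 or 3 casts the current game mode to GM_Blackjack and calls StartGame, PlayerHit or PlayerStand respectively.
; The actor holds no game logic itself and has an empty construction script.
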(event `Key|One`
  (params (Key :type "Key Structure"))
  (:`Pressed`
    (bind _asgm_blackjack (cast `/Game/Blueprints/Framework/GM_Blackjack` (`GameplayStatics.GetGameMode`)))
    (`BlackjackGameMode.StartGame` _asgm_blackjack)))

(event `Key|Two`
  (params (Key :type "Key Structure"))
  (:`Pressed`
    (bind _asgm_blackjack (cast `/Game/Blueprints/Framework/GM_Blackjack` (`GameplayStatics.GetGameMode`)))
    (`BlackjackGameMode.PlayerHit` _asgm_blackjack)))

(event `Key|Three`
  (params (Key :type "Key Structure"))
  (:`Pressed`
    (bind _asgm_blackjack (cast `/Game/Blueprints/Framework/GM_Blackjack` (`GameplayStatics.GetGameMode`)))
    (`BlackjackGameMode.PlayerStand` _asgm_blackjack)))

(fn `UserConstructionScript`)